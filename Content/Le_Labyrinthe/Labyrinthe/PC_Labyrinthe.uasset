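; Player controller for the Labyrinthe game that turns Enhanced Input actions into first-person character control.
; BeginPlay adds the move, mouse and vision mapping contexts and caches the player character as Adventurer for jumping.
; Movement follows control rotation, and look input drives controller yaw and pitch.
; The See action fires the character's ACViewLineTrace component, with both it and movement finding the character through GetActorOfClass rather than the cached reference.
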(event `self.ReceiveBeginPlay`
  (bind _returnvalue (pcsubsystem `EnhancedInputLocalPlayerSubsystem` self))
  ;[1 1 1] Mapping context
  (`/Engine/EditorBlueprintResources/StandardMacros.IsValid` _returnvalue
    (:`Is Valid`
      (`EnhancedInputSubsystemInterface.AddMappingContext` _returnvalue "/Game/Le_Labyrinthe/Inputs/IMC_Moves.IMC_Moves" 0 (struct))
      (`EnhancedInputSubsystemInterface.AddMappingContext` _returnvalue "/Game/Le_Labyrinthe/Inputs/IMC_Mouse.IMC_Mouse" 0 (struct))
      (`EnhancedInputSubsystemInterface.AddMappingContext` _returnvalue "/Game/Le_Labyrinthe/Inputs/IMC_Vision.IMC_Vision" 0 (struct))
      (bind _asbp_first_person_character (cast `/Game/Le_Labyrinthe/Blueprints/BP_FirstPersonCharacter` (`GameplayStatics.GetPlayerCharacter` 0)))
      (set `self.Adventurer` _asbp_first_person_character))))

(event `EnhancedInput|/Game/Le_Labyrinthe/Inputs/IA_Look`
  (params (ActionValue :type "Vector2D Structure") (ElapsedSeconds :type "Float (double-precision)") (TriggeredSeconds :type "Float (double-precision)") (InputAction :type "InputAction Object Reference" :default "/Game/Le_Labyrinthe/Inputs/IA_Look.IA_Look"))
  ;[1 1 1] PlayerLook
  (:`Triggered`
    (`self.AddYawInput` ActionValue_X)
    (`self.AddPitchInput` ActionValue_Y)))

(event `EnhancedInput|/Game/Le_Labyrinthe/Inputs/IA_Move`
  (params (ActionValue :type "Vector2D Structure") (ElapsedSeconds :type "Float (double-precision)") (TriggeredSeconds :type "Float (double-precision)") (InputAction :type "InputAction Object Reference" :default "/Game/Le_Labyrinthe/Inputs/IA_Move.IA_Move"))
  (bind (_returnvalue_roll _returnvalue_pitch _returnvalue_yaw) (`KismetMathLibrary.BreakRotator` (`self.GetControlRotation`)))
  ;[1 1 1] PlayerMovement
  (:`Triggered`
    (bind _returnvalue (`GameplayStatics.GetActorOfClass` "/Game/Le_Labyrinthe/Blueprints/BP_FirstPersonCharacter.BP_FirstPersonCharacter_C"))
    (`Pawn.AddMovementInput` _returnvalue (`KismetMathLibrary.GetRightVector` (`KismetMathLibrary.MakeRotator` _returnvalue_roll 0.0 _returnvalue_yaw)) ActionValue_X false)
    (`Pawn.AddMovementInput` _returnvalue (`KismetMathLibrary.GetForwardVector` (`KismetMathLibrary.MakeRotator` 0.0 0.0 _returnvalue_yaw)) ActionValue_Y false)))

(event `EnhancedInput|/Game/Le_Labyrinthe/Inputs/IA_See`
  (params (ActionValue :type Boolean) (ElapsedSeconds :type "Float (double-precision)") (TriggeredSeconds :type "Float (double-precision)") (InputAction :type "InputAction Object Reference" :default "/Game/Le_Labyrinthe/Inputs/IA_See.IA_See"))
  ;[1 1 1] ViewLineTrace
  (:`Started`
    (bind _returnvalue (`GameplayStatics.GetActorOfClass` "/Game/Le_Labyrinthe/Blueprints/BP_FirstPersonCharacter.BP_FirstPersonCharacter_C"))
    (`/Game/Le_Labyrinthe/Blueprints/Components/AC_ViewLineTrace.CastViewLineTrace` (`/Game/Le_Labyrinthe/Blueprints/BP_FirstPersonCharacter.AC_ViewLineTrace` _returnvalue))))

(event `EnhancedInput|/Game/Le_Labyrinthe/Inputs/IA_Jump`
  (params (ActionValue :type Boolean) (ElapsedSeconds :type "Float (double-precision)") (TriggeredSeconds :type "Float (double-precision)") (InputAction :type "InputAction Object Reference" :default "/Game/Le_Labyrinthe/Inputs/IA_Jump.IA_Jump"))
  (bind _adventurer (`self.Adventurer`))
  ;[1 1 1] PlayerMovement
  (:`Started`
    (`Character.Jump` _adventurer))
  (:`Completed`
    (`Character.StopJumping` _adventurer)))

(fn `UserConstructionScript`)