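; Actor component for a labyrinth puzzle that opens a secret passage through objects the player looks at.
; CastViewLineTrace fires a debug-drawn trace 1000 units along the camera view and identifies the hit actor by display name.
; An "Interruptor" is destroyed, a "BP_Torche" gets a fire particle, and both increment a shared counter.
; At two, it destroys the "Passage Secret" static mesh; repeated torch hits also count.
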(event `CastViewLineTrace`
  (bind _returnvalue (`GameplayStatics.GetPlayerCameraManager` 0))
  (bind _hitobjectname (`self.HitObjectName`))
  (bind _returnvalue_2 (`SceneComponent.K2_GetComponentLocation` (`Actor.RootComponent` _returnvalue)))
  ;[1 1 1] Launch the line trace
  (bind _outhit (`KismetSystemLibrary.LineTraceSingle` :`Start` _returnvalue_2 :`End` (+ _returnvalue_2 (* (`Actor.GetActorForwardVector` _returnvalue) 1000.0)) :`TraceChannel` "TraceTypeQuery4" :`DrawDebugType` "Persistent"))
  ;[1 1 1] Check if the object that has been hitted is the Torch, the Interruptor or something else
  (bind _output_get (set `self.ObjectHit` (`.HitActor` (`GameplayStatics.BreakHitResult` _outhit))))
  (bind _returnvalue_3 (`KismetSystemLibrary.GetDisplayName` _output_get))
  (`KismetSystemLibrary.PrintString` _returnvalue_3)
  (set `self.HitObjectName` _returnvalue_3)
  (if (`KismetStringLibrary.EqualEqual_StrStr` _hitobjectname "Interruptor")
    (`KismetSystemLibrary.PrintString` "Interruptor Activated")
    (`Actor.K2_DestroyActor` (`self.ObjectHit`))
    ;;[1 1 1] If var = 2 => Door can Open
    (set `self.DoorCanBeOpened` (+ (`self.DoorCanBeOpened`) 1) :!label _label)
    (if (== (`self.DoorCanBeOpened`) 2)
      (bind _outactors (`GameplayStatics.GetAllActorsOfClass` "/Script/Engine.StaticMeshActor"))
      (for _array_element _outactors
        (if (`KismetStringLibrary.EqualEqual_StrStr` (`KismetSystemLibrary.GetDisplayName` _array_element) "Passage Secret")
          (`Actor.K2_DestroyActor` _array_element)
          (break))))
    (elif (`KismetStringLibrary.EqualEqual_StrStr` _hitobjectname "BP_Torche")
      (`KismetSystemLibrary.PrintString` "Torch Activated")
      (`ParticleSystemComponent.SetTemplate` (`Actor.GetComponentByClass` (`self.ObjectHit`) "/Script/Engine.ParticleSystemComponent") "/Game/StarterContent/Particles/P_Fire.P_Fire")
      (goto _label))))