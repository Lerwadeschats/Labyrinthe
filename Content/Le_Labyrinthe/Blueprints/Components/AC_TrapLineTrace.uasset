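; AC_TrapLineTrace is an actor component that gives a labyrinth trap a line-trace trigger.
; When CastTrapLineTrace is called, it traces from the owner's root location along its right vector on a custom trace channel, with persistent debug drawing.
; On a hit it prints a placeholder "trap activated" message and destroys the owning actor rather than applying damage or killing anyone.
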(event `CastTrapLineTrace`
  (bind _returnvalue (`self.GetOwner`))
  (bind _returnvalue_2 (`SceneComponent.K2_GetComponentLocation` (`Actor.RootComponent` _returnvalue)))
  (bind (_outhit _returnvalue_3) (`KismetSystemLibrary.LineTraceSingle` :`Start` _returnvalue_2 :`End` (+ _returnvalue_2 (* (`Actor.GetActorRightVector` _returnvalue) 2000.0)) :`TraceChannel` "TraceTypeQuery3" :`DrawDebugType` "Persistent" :`TraceColor` (struct :`G` 0.245152 :`B` 1.0 :`A` 1.0)))
  (if _returnvalue_3
    (`KismetSystemLibrary.PrintString` "Trap activated (You're supposed to be dead but I'm kind you know? :P" true true (struct :`G` 0.66 :`B` 1.0 :`A` 1.0) 10.0)
    (`Actor.K2_DestroyActor` (`self.GetOwner`))))